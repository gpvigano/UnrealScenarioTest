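; BP_CircuitCable is a cable actor that visually links the leads of two circuit components.
; ConnectComponentLeads stores both leads and calls UpdateCable, which moves the actor to the start lead's SolderSocket and sets the cable's local-space end at the other lead's socket.
; Cable length is the socket distance scaled by LengthFactor.
; Disconnect only clears the lead references, and nothing updates on Tick.
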(event EventBeginPlay)

(event Collision|EventActorBeginOverlap
  (params (OtherActor :type Actor%20Object%20Reference)))

(event EventTick
  (params (DeltaSeconds :type Float%20%28single-precision%29)))

(fn ConstructionScript)

(fn ConnectComponentLeads
  (params (StartSceneComponent :type Scene%20Component%20Object%20Reference) (EndSceneComponent :type Scene%20Component%20Object%20Reference))
  (Variables|Default|SetStartLead StartSceneComponent)
  (Variables|Default|SetEndLead EndSceneComponent)
  (CallFunction|UpdateCable))

(fn UpdateCable
  (Utilities|IsValid (Variables|Default|GetStartLead)
    (:Is%20Valid
      (Variables|Default|SetStartPos (Transformation|GetSocketLocation (Variables|Default|GetStartLead) "SolderSocket")))
    (:Is%20Not%20Valid
      _))
  (Transformation|SetActorLocation (Variables|Default|GetStartPos) false true)
  (Utilities|IsValid (Variables|Default|GetEndLead)
    (:Is%20Valid
      (Variables|Default|SetEndPos (Transformation|GetSocketLocation (Variables|Default|GetEndLead) "SolderSocket")))
    (:Is%20Not%20Valid
      _))
  (Variables|/Script/CableComponent.CableComponent|SetEndLocation (Variables|Default|GetCableComponent) (Math|Transform|InverseTransformLocation (Transformation|GetWorldTransform (Variables|Default|GetCableComponent)) (Variables|Default|GetEndPos)))
  (Variables|/Script/CableComponent.CableComponent|SetCableLength (Variables|Default|GetCableComponent) (CallFunction|CalculateLength (Variables|Default|GetEndPos) (Variables|Default|GetStartPos)))
  (return))

(fn CalculateLength
  (params (A :type Vector) (B :type Vector))
  (return (* (Math|Vector|VectorLength (- A B)) (Variables|Default|GetLengthFactor))))

(fn Disconnect
  (Variables|Default|SetStartLead 0)
  (Variables|Default|SetEndLead 0)
  (return))
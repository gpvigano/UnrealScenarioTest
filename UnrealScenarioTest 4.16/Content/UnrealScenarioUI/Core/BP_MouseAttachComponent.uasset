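; BP_MouseAttachComponent is a component that makes an actor follow the mouse cursor in the world.
; Each tick it falls back to its owner when no valid Target is set, then calls MouseDragLocation with the first player controller and a Distance.
; When that call succeeds, it moves the Target straight to the returned location without sweeping.
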(event EventBeginPlay)

(event EventTick
  (params (DeltaSeconds :type Float%20%28single-precision%29))
  (Utilities|IsValid (Variables|Default|GetTarget)
    (:Is%20Valid
      _)
    (:Is%20Not%20Valid
      (Variables|Default|SetTarget (Components|GetOwner))))
  (Utilities|IsValid (Variables|Default|GetTarget)
    (:Is%20Valid
      (bind (_location _returnvalue) (Class|UEUtil|MouseDragLocation (Game|GetPlayerController 0) (Variables|Default|GetDistance)))
      (if _returnvalue
        (Transformation|SetActorLocation (Variables|Default|GetTarget) _location false false)))))